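; BP_WaterQualityTest is a build item that acts as a test readout for the water system.
; Its Waterin event receives water quality and pressure and writes them to text render components.
; It then line traces 100 units upward on Visibility, showing the Durability of any BP_ParentWaterItemDurability actor hit, or fallback text when the cast fails.
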(event EventWaterin
  (params (Box :type String) (WaterQuality :type Integer) (WaterPressure :type Float%20%28single-precision%29))
  (bind _returnvalue (Transformation|GetActorLocation))
  (bind _textrender5 (Variables|Default|GetTextRender5))
  (Rendering|Components|TextRender|SetText (Variables|Default|GetTextRender) (Utilities|Text|ToText(Integer) WaterQuality))
  (Rendering|Components|TextRender|SetText (Variables|Default|GetTextRender2) (Utilities|Text|ToText(Float) WaterPressure "HalfToEven"))
  (bind _outhit (Collision|LineTraceByChannel (Transformation|GetActorLocation) (Math|Vector|MakeVector (.x _returnvalue) (.y _returnvalue) (+ (.z _returnvalue) 1e+02)) "TraceTypeQuery1" false 0 "None"))
  (bind _asbp_parent_water_item_durability (Utilities|Casting|CastToBP_ParentWaterItemDurability (.HitActor (Collision|BreakHitResult _outhit)))
    (:then
      (Rendering|Components|TextRender|SetText _textrender5 (Utilities|Text|ToText(Float) (Variables|/Game/WorldObjects/Items/BuildItems/BP_ParentWaterItemDurability.BP_ParentWaterItemDurability_C|GetDurability _asbp_parent_water_item_durability) "HalfToEven")))
    (:CastFailed
      (Rendering|Components|TextRender|SetText _textrender5 (Variables|Default|GetNewVar_0)))))

(fn ConstructionScript
  (|CallParentFunction))