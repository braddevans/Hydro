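; BP_StraightPipe is a buildable straight pipe item that reacts to incoming water through its Waterin override.
; The override switches on the input box with empty branches, and a short visibility trace runs from the center point along its right vector.
; It also binds and immediately calls a WaterPress dispatcher, whose handler gathers all BP_Water actors.
; The trace and actor results are unused, so the flow logic appears unfinished.
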(event Custom|CustomEvent_0
  (Actor|GetAllActorsOfClass "/Game/WorldObjects/BP_Water.BP_Water_C"))

(event EventOverrideWaterin
  (params (Box :type String))
  (bind _centerpoint (Variables|Default|GetCenterPoint))
  (bind _returnvalue (Transformation|GetWorldLocation _centerpoint))
  (switch string Box
    (:Default
      _)
    (:Box1
      _)
    (:Box2
      _))
  (Collision|LineTraceByChannel _returnvalue (+ (* (Math|Vector|GetRightVector _centerpoint) 52.0) _returnvalue) "TraceTypeQuery1" false 0 "None")
  (EventDispatchers|BindEventtoWaterPress (delegate Custom|CustomEvent_0))
  (Default|CallWaterPress))

(fn ConstructionScript
  (|CallParentFunction))