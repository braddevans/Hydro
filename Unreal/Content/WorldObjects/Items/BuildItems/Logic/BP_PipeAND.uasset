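; BP_PipeAND is a T-shaped buildable pipe that acts as an AND gate, passing water on only when at least two of its three boxes receive it.
; Each Waterin event flags its box, then SendWater outputs through the unflagged one at one less pressure.
; A 0.95-second timer clears the gate state, while a restarted 1.5-second timer resets the text displays of pressure, quality and direction once water stops.
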(event Custom|CustomEvent_0
  (Variables|Default|SetWaterOut? false)
  (Variables|Default|SetWaterIn? false)
  (Variables|Default|SetInputs (Variables|Default|GetDefaults)))

(event Custom|CustomEvent_1
  (bind _returnvalue (Utilities|Text|ToText(String) "---"))
  (if (not (Variables|Default|GetWaterIn?))
    (Variables|Default|SetCounter 0)
    (Rendering|Components|TextRender|SetText (Variables|Default|GetTextRender10) (Utilities|Array|Get(acopy) (Variables|Default|GetDirections) 3))
    (Rendering|Components|TextRender|SetText (Variables|Default|GetTextRender5) _returnvalue)
    (Rendering|Components|TextRender|SetText (Variables|Default|GetTextRender6) _returnvalue)))

(event EventWaterin
  (params (Box :type String) (WaterQuality :type Integer) (WaterPressure :type Float%20%28single-precision%29))
  (bind _returnvalue (- WaterPressure 1.0))
  (bind _inputs (Variables|Default|GetInputs))
  (if (not (Variables|Default|GetWaterOut?))
    (if (Variables|Default|GetWaterIn?)
      _
      (else
        (Utilities|Time|SetTimerbyEvent (delegate Custom|CustomEvent_0) 0.95)
        (Variables|Default|SetWaterIn? true)))
    (Utilities|Time|SetTimerbyEvent (delegate Custom|CustomEvent_1) 1.5)
    (Variables|Default|SetCounter 0)
    (Rendering|Components|TextRender|SetText (Variables|Default|GetTextRender5) (Utilities|Text|ToText(Float) _returnvalue "HalfToEven"))
    (Rendering|Components|TextRender|SetText (Variables|Default|GetTextRender6) (Utilities|Text|ToText(Integer) WaterQuality))
    (switch string Box
      (:Box1
        (Utilities|Array|SetArrayElem _inputs 0 true))
      (:Box2
        (Utilities|Array|SetArrayElem _inputs 1 true))
      (:Box3
        (Utilities|Array|SetArrayElem _inputs 2 true)))
    (for (_array_element _array_index) _inputs
      (if _array_element
        (bind _output_get (Variables|Default|SetCounter (+ (Variables|Default|GetCounter) 1)))
        (Rendering|Components|TextRender|SetText (Variables|Default|GetTextRender_0) (Utilities|Text|ToText(Integer) _output_get))
        (else
          (Variables|Default|SetEmptyPipe _array_index))))
    (if (>= (Variables|Default|GetCounter) 2)
      (CallFunction|SendWater (Utilities|Array|Get(acopy) (Variables|Default|GetBoxArray) (Variables|Default|GetEmptyPipe)) WaterQuality _returnvalue)
      (Variables|Default|SetWaterOut? true)
      (Rendering|Components|TextRender|SetText (Variables|Default|GetTextRender10) (Utilities|Array|Get(acopy) (Variables|Default|GetDirections) (Variables|Default|GetEmptyPipe))))))

(fn ConstructionScript
  (|CallParentFunction)
  (Components|StaticMesh|SetStaticMesh (Variables|Default|GetStaticMesh) "/Game/Meshes/UsedItems/Build/SM_PipeT.SM_PipeT")
  (Transformation|SetRelativeLocation (Variables|Default|GetBox3) "50.000000, 0, 0" false false))