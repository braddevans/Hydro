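; BP_PipeXOR is a T-shaped pipe build item that acts as an XOR logic gate for water flow.
; Waterin flags which input box received water and starts a one-second timer to evaluate the inputs.
; If exactly one is flagged, water is sent on with pressure reduced by one, then inputs reset.
; Text renders show pressure, quality and direction, with a second timer clearing them when flow stops.
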(event Custom|CustomEvent_0
  (Variables|Default|SetCounter 0)
  (Variables|Default|SetWaterIn? false)
  (for _array_element (Variables|Default|GetInputs)
    (if _array_element
      (Variables|Default|SetCounter (+ (Variables|Default|GetCounter) 1))
      (Rendering|Components|TextRender|SetText (Variables|Default|GetTextRender) (Utilities|Text|ToText(Integer) 0))))
  (if (== (Variables|Default|GetCounter) 1)
    (CallFunction|SendWater (Variables|Default|GetBox3_0) (stale EventWaterin WaterQuality) (- (stale EventWaterin WaterPressure) 1.0))
    (Rendering|Components|TextRender|SetText (Variables|Default|GetTextRender10) (Utilities|Array|Get(acopy) (Variables|Default|GetDirections) 2)))
  (Variables|Default|SetInputs (Variables|Default|GetDefaults)))

(event Custom|CustomEvent_1
  (bind _returnvalue (Utilities|Text|ToText(String) "---"))
  (if (not (Variables|Default|GetWaterIn?))
    (Rendering|Components|TextRender|SetText (Variables|Default|GetTextRender10) (Utilities|Array|Get(acopy) (Variables|Default|GetDirections) 3))
    (Rendering|Components|TextRender|SetText (Variables|Default|GetTextRender5) _returnvalue)
    (Rendering|Components|TextRender|SetText (Variables|Default|GetTextRender6) _returnvalue)))

(event EventWaterin
  (params (Box :type String) (WaterQuality :type Integer) (WaterPressure :type Float%20%28single-precision%29))
  (bind _inputs (Variables|Default|GetInputs))
  (if (Variables|Default|GetWaterIn?)
    _
    (else
      (Utilities|Time|SetTimerbyEvent (delegate Custom|CustomEvent_0) 1.0)
      (Variables|Default|SetWaterIn? true)))
  (Utilities|Time|SetTimerbyEvent (delegate Custom|CustomEvent_1) 1.5)
  (Rendering|Components|TextRender|SetText (Variables|Default|GetTextRender5) (Utilities|Text|ToText(Float) (- WaterPressure 1.0) "HalfToEven"))
  (Rendering|Components|TextRender|SetText (Variables|Default|GetTextRender6) (Utilities|Text|ToText(Integer) WaterQuality))
  (switch string Box
    (:Box1
      (Utilities|Array|SetArrayElem _inputs 0 false))
    (:Box2
      (Utilities|Array|SetArrayElem _inputs 1 false))
    (:Box3
      (Utilities|Array|SetArrayElem _inputs 2 false))))

(fn ConstructionScript
  (|CallParentFunction)
  (Components|StaticMesh|SetStaticMesh (Variables|Default|GetStaticMesh) "/Game/Meshes/UsedItems/Build/SM_PipeT.SM_PipeT"))