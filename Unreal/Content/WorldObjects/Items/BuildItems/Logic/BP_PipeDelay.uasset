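; BP_PipeDelay is a straight pipe build item that relays water between its two ends, showing flow direction, pressure and quality on text renders.
; Water entering either box is sent immediately out of the other with pressure reduced by one.
; In/out flags block further relays until a 0.95-second timer clears them.
; A 1.5-second timer, restarted on each accepted inflow, blanks the readout when no water is flagged.
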(event Custom|CustomEvent_0
  (Variables|Default|SetWaterOut? false)
  (Variables|Default|SetWaterIn? false))

(event Custom|CustomEvent_1
  (bind _returnvalue (Utilities|Text|ToText(String) "---"))
  (if (not (Variables|Default|GetWaterIn?))
    (Rendering|Components|TextRender|SetText (Variables|Default|GetTextRender10) (Utilities|Array|Get(acopy) (Variables|Default|GetDirections) 3))
    (Rendering|Components|TextRender|SetText (Variables|Default|GetTextRender5) _returnvalue)
    (Rendering|Components|TextRender|SetText (Variables|Default|GetTextRender6) _returnvalue)))

(event EventWaterin
  (params (Box :type String) (WaterQuality :type Integer) (WaterPressure :type Float%20%28single-precision%29))
  (bind _returnvalue (- WaterPressure 1.0))
  (bind _inputs (Variables|Default|GetInputs))
  (bind _directions (Variables|Default|GetDirections))
  (bind _textrender10 (Variables|Default|GetTextRender10))
  (if (not (Variables|Default|GetWaterOut?))
    (if (Variables|Default|GetWaterIn?)
      _
      (else
        (Utilities|Time|SetTimerbyEvent (delegate Custom|CustomEvent_0) 0.95)
        (Variables|Default|SetWaterIn? true)))
    (Utilities|Time|SetTimerbyEvent (delegate Custom|CustomEvent_1) 1.5)
    (Rendering|Components|TextRender|SetText (Variables|Default|GetTextRender5) (Utilities|Text|ToText(Float) _returnvalue "HalfToEven"))
    (Rendering|Components|TextRender|SetText (Variables|Default|GetTextRender6) (Utilities|Text|ToText(Integer) WaterQuality))
    (switch string Box
      (:Box1
        (Utilities|Array|SetArrayElem _inputs 0 true)
        (CallFunction|SendWater (Variables|Default|GetBox2) WaterQuality _returnvalue)
        (Rendering|Components|TextRender|SetText _textrender10 (Utilities|Array|Get(acopy) _directions 1)))
      (:Box2
        (Utilities|Array|SetArrayElem _inputs 1 true)
        (CallFunction|SendWater (Variables|Default|GetBox1) WaterQuality _returnvalue)
        (Rendering|Components|TextRender|SetText _textrender10 (Utilities|Array|Get(acopy) _directions))))
    (Variables|Default|SetWaterOut? true)))

(fn ConstructionScript
  (|CallParentFunction)
  (Components|StaticMesh|SetStaticMesh (Variables|Default|GetStaticMesh) "/Game/Meshes/UsedItems/Build/SM_PipeStraight.SM_PipeStraight"))