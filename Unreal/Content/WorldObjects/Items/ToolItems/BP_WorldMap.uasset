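; World map actor that toggles the map widget and doubles as a host for debug cheats.
; BeginPlay creates the hidden cheat menu and map widgets and enables input; F7 and OpenMap toggle them.
; Tick drives vertical flight from held inputs and pins the day/night hour while TimeFreeze is checked.
; Other inputs zero player velocity, repeatedly generate gems in the closest pan, or clone the screen-center item as paid-for.
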(event Custom|CustomEvent_0
  (Default|GenerateGems (stale Input|KeyboardEvents|F3 _asbp_pan)))

(event EventTick
  (params (DeltaSeconds :type Float%20%28single-precision%29))
  (bind _returnvalue (Game|GetPlayerCharacter 0))
  (bind _returnvalue_2 (Game|Player|GetPlayerPawn 0))
  (bind _cheatmenu (Variables|Default|GetCheatMenu))
  (bind _charactermovement (Variables|/Script/Engine.Character|GetCharacterMovement _returnvalue))
  (bind _maxacceleration (Variables|/Script/Engine.CharacterMovementComponent|GetMaxAcceleration _charactermovement))
  (Utilities|FlowControl|Sequence
    (:then_0
      ;[1 1 1] Flight
      (if (Variables|Default|GetShiftHeld?)
        (Pawn|Input|AddMovementInput _returnvalue_2 (Math|Vector|MakeVector 0.0 0.0 _maxacceleration) 1e+02 false)
        (elif (Variables|Default|GetCtrlHeld?)
          (Pawn|Input|AddMovementInput _returnvalue_2 (Math|Vector|MakeVector 0.0 0.0 (* _maxacceleration -1.0)) 1e+02 false))))
    (:then_1
      (if (Class|CheckBox|IsChecked (Variables|/Game/CheatMenu/CheatMenu.CheatMenu_C|GetTimeFreeze _cheatmenu))
        (Variables|/Game/WorldObjects/BP_DayNightCycle.BP_DayNightCycle_C|SetHour (Variables|/Game/CheatMenu/CheatMenu.CheatMenu_C|GetDayNight _cheatmenu) (Variables|/Game/CheatMenu/CheatMenu.CheatMenu_C|GetHour _cheatmenu))))))

(event EventBeginPlay
  (bind _returnvalue (Game|GetPlayerController 0))
  ;[1 1 1] Setup
  (Actor|SetOwner _returnvalue)
  (if (not (Utilities|IsValid (Variables|Default|GetCheatMenu)))
    (bind _returnvalue_2 (UserInterface|CreateWidget "/Game/CheatMenu/CheatMenu.CheatMenu_C" 0 0 0 "Unchecked" "Boop"))
    (bind _output_get (Variables|Default|SetCheatMenu _returnvalue_2))
    (UserInterface|Viewport|AddtoViewport _output_get 0)
    (Input|EnableInput _returnvalue)
    (Widget|SetVisibility _output_get "Collapsed")
    (if (not (Utilities|IsValid (Variables|Default|GetWorldMap)))
      (bind _returnvalue_3 (UserInterface|CreateWidget "/Game/UI/UI_WorldMap.UI_WorldMap_C"))
      (bind _output_get_2 (Variables|Default|SetWorldMap _returnvalue_3))
      (UserInterface|Viewport|AddtoViewport _output_get_2 0)
      (Widget|SetVisibility _output_get_2 "Collapsed"))))

(event Input|ActionEvents|InputActionOpenMap
  (params (Key :type Key%20Structure))
  (bind _worldmap (Variables|Default|GetWorldMap))
  ;[1 1 1] Map
  (:Pressed
    (if (Widget|IsVisible _worldmap)
      (Widget|SetVisibility _worldmap "Collapsed")
      (else
        (Widget|SetVisibility _worldmap "Visible")))))

(event Input|ActionEvents|InputActionCloneItem
  (params (Key :type Key%20Structure))
  (bind _returnvalue (Game|Player|GetPlayerPawn 0))
  (bind _returnvalue_2 (Game|GetPlayerController 0))
  (bind _returnvalue_3 (Transformation|GetActorLocation _returnvalue))
  (bind _hitresult (Game|Player|GetHitResultUnderCursorbyChannel _returnvalue_2 "TraceTypeQuery1" true))
  (bind (_bblockinghit _binitialoverlap _time _distance _location _impactpoint _normal _impactnormal _physmat _hitactor) (Collision|BreakHitResult _hitresult))
  ;[1 1 1] Duplicate Items
  (:Pressed
    (bind _returnvalue_4 (Settings|GetGameUserSettings))
    (Class|PlayerController|SetMouseLocation (Game|GetPlayerController 0) (/ (.x (Class|GameUserSettings|GetScreenResolution _returnvalue_4)) 2) (/ (.y (Class|GameUserSettings|GetScreenResolution _returnvalue_4)) 2))
    (Utilities|Casting|CastToBP_ParentItem _hitactor)
    (bind _returnvalue_5 (Game|SpawnActorfromClass (Utilities|GetClass _hitactor) (Math|Transform|MakeTransform (Math|Vector|MakeVector (+ (/ (- (.x _location) (.x _returnvalue_3)) 2.0) (.x _returnvalue_3)) (+ (/ (- (.y _location) (.y _returnvalue_3)) 2.0) (.y _returnvalue_3)) (+ (/ (- (.z _location) (.z _returnvalue_3)) 2.0) (.z _returnvalue_3))) "0, 0, 0" "1,1,1") "AdjustIfPossibleButAlwaysSpawn" _returnvalue_2 0))
    (bind _asbp_parent_item (Utilities|Casting|CastToBP_ParentItem _returnvalue_5))
    (Variables|/Game/WorldObjects/Items/BP_ParentItem.BP_ParentItem_C|SetPaidFor? _asbp_parent_item true)))

(event Input|ActionEvents|InputActionPlayerStop
  (params (Key :type Key%20Structure))
  ;[1 1 1] Flight
  (:Pressed
    (Variables|/Script/Engine.MovementComponent|SetVelocity (Variables|/Script/Engine.Character|GetCharacterMovement (Game|GetPlayerCharacter 0)) "0, 0, 0")))

(event Input|ActionEvents|InputActionPlayerUp
  (params (Key :type Key%20Structure))
  ;[1 1 1] Flight
  (:Pressed
    (Variables|Default|SetShiftHeld? true))
  (:Released
    (Variables|Default|SetShiftHeld? false)))

(event Input|ActionEvents|InputActionPlayerDown
  (params (Key :type Key%20Structure))
  ;[1 1 1] Flight
  (:Pressed
    (Variables|Default|SetCtrlHeld? true))
  (:Released
    (Variables|Default|SetCtrlHeld? false)))

(event Input|KeyboardEvents|F3
  (params (Key :type Key%20Structure))
  (:Pressed
    (bind _newparam1 (Default|GetClosestObject (Variables|Default|GetCheatMenu) "/Game/WorldObjects/Items/ToolItems/BP_Pan.BP_Pan_C"))
    (bind _asbp_pan (Utilities|Casting|CastToBP_Pan _newparam1))
    (bind _returnvalue (Utilities|Time|SetTimerbyEvent (delegate Custom|CustomEvent_0) 0.01 true)))
  (:Released
    (Utilities|Time|ClearandInvalidateTimerbyHandle _returnvalue)))

(event Input|KeyboardEvents|F7
  (params (Key :type Key%20Structure))
  (bind _cheatmenu (Variables|Default|GetCheatMenu))
  ;[1 1 1] Cheat Menu
  (:Pressed
    (if (Widget|IsVisible _cheatmenu)
      (Default|ResetVis _cheatmenu)
      (Variables|/Script/Engine.PlayerController|SetbShowMouseCursor (Game|GetPlayerController 0) false)
      (else
        (Widget|SetVisibility _cheatmenu "Visible")
        (Variables|/Script/Engine.PlayerController|SetbShowMouseCursor (Game|GetPlayerController 0) true)))))

(fn ConstructionScript
  (|CallParentFunction))